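; BP_Ryo is a character Blueprint with keyboard bindings that directly change life and stamina, apparently for testing those stats.
; Q applies damage, R heals both life and stamina, F drains stamina and X drains life.
; Each key first requires player character 0 to cast to BP_Ryo, then calls stat functions that are not defined in these graphs.
; The construction script is empty.
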(event Input|KeyboardEvents|Q
  (params (Key :type Key%20Structure :default "None"))
  (:Pressed
    (Utilities|Casting|CastToBP_Ryo (Game|GetPlayerCharacter 0))
    (Class|CharacterCommon|SetDamage 1e+01)))

(event Input|KeyboardEvents|R
  (params (Key :type Key%20Structure :default "None"))
  (:Pressed
    (Utilities|Casting|CastToBP_Ryo (Game|GetPlayerCharacter 0))
    (Class|CharacterCommon|HealLife 1e+01)
    (Class|CharacterCommon|HealStamina 1.0)))

(event Input|KeyboardEvents|F
  (params (Key :type Key%20Structure :default "None"))
  (:Pressed
    (Utilities|Casting|CastToBP_Ryo (Game|GetPlayerCharacter 0))
    (Class|CharacterCommon|DrainStamina)))

(event Input|KeyboardEvents|X
  (params (Key :type Key%20Structure :default "None"))
  (:Pressed
    (Utilities|Casting|CastToBP_Ryo (Game|GetPlayerCharacter 0))
    (Class|CharacterCommon|DrainLife)))

(fn ConstructionScript)