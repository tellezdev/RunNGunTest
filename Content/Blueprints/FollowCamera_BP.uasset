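; Camera zone actor that blends the player's view to its own camera when BP_CharacterKen overlaps its ActorCollision box.
; The construction script sets the camera's transform and projection, plus the bound and trigger boxes, from per-instance variables.
; Despite the name, the camera does not follow: Tick is empty, and the interpolated X/Z follow clamped to CameraBoundBox is disconnected.
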(event OnComponentBeginOverlap(ActorCollision)
  (params (OverlappedComponent :type Primitive%20Component%20Object%20Reference) (OtherActor :type Actor%20Object%20Reference) (OtherComp :type Primitive%20Component%20Object%20Reference) (OtherBodyIndex :type Integer) (bFromSweep :type Boolean) (SweepResult :type Hit%20Result%20Structure%20%28by%20ref%29))
  (Utilities|Casting|CastToBP_CharacterKen OtherActor)
  (Game|Player|SetViewTargetwithBlend (Game|GetPlayerController 0) self (Variables|CameraView|GetBlendTime) (Variables|CameraView|GetBlendFunc) (Variables|CameraView|GetBlendExp) false))

(event EventTick
  (params (DeltaSeconds :type Float%20%28single-precision%29)))

(fn ConstructionScript
  (bind _cameraboxtransform (Variables|CameraBounds|GetCameraBoxTransform))
  (Utilities|FlowControl|Sequence
    (:then_0
      (Transformation|SetRelativeTransform (Variables|Default|GetCamera) (Variables|CameraView|GetCameraTransform) false false)
      (Camera|SetFieldOfView (Variables|Default|GetCamera) (Variables|CameraView|GetFoV))
      (Class|CameraComponent|SetProjectionMode (Variables|Default|GetCamera) (Variables|CameraView|GetProjectionMode))
      (Class|CameraComponent|SetOrthoWidth (Variables|Default|GetCamera) (Variables|CameraView|GetOrthoWidth)))
    (:then_1
      (Transformation|SetRelativeTransform (Variables|Default|GetCameraBoundBox) (Math|Transform|MakeTransform (Math|Vector|MakeVector (.x (.location _cameraboxtransform)) (.y (.location _cameraboxtransform)) (- (.z (.location _cameraboxtransform)) -5e+01)) (.rotation _cameraboxtransform) (.scale _cameraboxtransform)) false false)
      (Components|Box|SetBoxExtent (Variables|Default|GetCameraBoundBox) (Variables|CameraBounds|GetCameraBoxExtent) true))
    (:then_2
      (Transformation|SetRelativeTransform (Variables|Default|GetActorCollision) (Variables|CameraBounds|GetActorCollisionTransform) false false)
      (Components|Box|SetBoxExtent (Variables|Default|GetActorCollision) (Variables|CameraBounds|GetActorCollisionExtent) true))))