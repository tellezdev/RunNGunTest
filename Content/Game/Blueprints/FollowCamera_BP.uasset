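; FollowCamera_BP is a zone camera that takes over the player's view when BP_CharacterKen enters its collision box.
; The overlap blends the view target to this actor.
; Each tick, the camera eases toward the pawn in X and Z, clamped to CameraBoundBox with Y unchanged, or snaps to a hard-coded position without a valid pawn.
; The construction script applies exposed transforms, extents and projection settings to the camera and both boxes.
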(event OnComponentBeginOverlap(ActorCollision)
  (params (OverlappedComponent :type Primitive%20Component%20Object%20Reference) (OtherActor :type Actor%20Object%20Reference) (OtherComp :type Primitive%20Component%20Object%20Reference) (OtherBodyIndex :type Integer) (bFromSweep :type Boolean) (SweepResult :type Hit%20Result%20Structure%20%28by%20ref%29))
  (Utilities|Casting|CastToBP_CharacterKen OtherActor)
  (Game|Player|SetViewTargetwithBlend (Game|GetPlayerController 0) self (Variables|CameraView|GetBlendTime) (Variables|CameraView|GetBlendFunc) (Variables|CameraView|GetBlendExp) false))

(event EventTick
  (params (DeltaSeconds :type Float%20%28single-precision%29))
  (bind _returnvalue (Game|Player|GetPlayerPawn 0))
  (bind _cameraboundbox (Variables|Default|GetCameraBoundBox))
  (bind _returnvalue_2 (Transformation|GetActorLocation _returnvalue))
  (bind (_origin _boxextent) (Collision|GetComponentBounds _cameraboundbox))
  (bind _returnvalue_3 (- _origin _boxextent))
  (bind _returnvalue_4 (+ _origin _boxextent))
  (Utilities|IsValid _returnvalue
    (:Is%20Valid
      (Transformation|SetWorldLocation (Variables|Default|GetCamera) (Math|Interpolation|VInterpTo (Transformation|GetWorldLocation (Variables|Default|GetCamera)) (Math|Vector|MakeVector (Math|Float|Clamp(Float) (.x _returnvalue_2) (.x _returnvalue_3) (.x _returnvalue_4)) (.y (Transformation|GetWorldLocation (Variables|Default|GetCamera))) (Math|Float|Clamp(Float) (.z _returnvalue_2) (.z _returnvalue_3) (.z _returnvalue_4))) (Utilities|Time|GetWorldDeltaSeconds) 5.0) false false))
    (:Is%20Not%20Valid
      (Transformation|SetWorldLocation (Variables|Default|GetCamera) "-2064.000000,0.000000,1339.000000" false false))))

(fn ConstructionScript
  (bind _cameraboxtransform (Variables|CameraBounds|GetCameraBoxTransform))
  (Utilities|FlowControl|Sequence
    (:then_0
      (Transformation|SetRelativeTransform (Variables|Default|GetCamera) (Variables|CameraView|GetCameraTransform) false false)
      (Camera|SetFieldOfView (Variables|Default|GetCamera) (Variables|CameraView|GetFoV))
      (Class|CameraComponent|SetProjectionMode (Variables|Default|GetCamera) (Variables|CameraView|GetProjectionMode))
      (Class|CameraComponent|SetOrthoWidth (Variables|Default|GetCamera) (Variables|CameraView|GetOrthoWidth)))
    (:then_1
      (Transformation|SetRelativeTransform (Variables|Default|GetCameraBoundBox) (Math|Transform|MakeTransform (Math|Vector|MakeVector (.x (.location _cameraboxtransform)) (.y (.location _cameraboxtransform)) (- (.z (.location _cameraboxtransform)) -5e+01)) (.rotation _cameraboxtransform) (.scale _cameraboxtransform)) false false)
      (Components|Box|SetBoxExtent (Variables|Default|GetCameraBoundBox) (Variables|CameraBounds|GetCameraBoxExtent) true))
    (:then_2
      (Transformation|SetRelativeTransform (Variables|Default|GetActorCollision) (Variables|CameraBounds|GetActorCollisionTransform) false false)
      (Components|Box|SetBoxExtent (Variables|Default|GetActorCollision) (Variables|CameraBounds|GetActorCollisionExtent) true))))